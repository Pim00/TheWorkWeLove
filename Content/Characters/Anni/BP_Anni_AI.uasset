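; BP_Anni_AI is the AI controller for the Anni character, starting a behavior tree on play and feeding it perception data through the blackboard.
; Sight of the player pawn sets TargetActor, while losing sight clears it and stores the stimulus position as LastSeenLocation.
; Hearing stimuli from any actor write their position to HearingNoiseLocation.
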(event `self.ReceiveBeginPlay`
  (`self.RunBehaviorTree` null))

(event `self.AIPerception.OnTargetPerceptionUpdated`
  (params (Actor :type "Actor Object Reference") (Stimulus :type "AIStimulus Structure"))
  (bind (_age _expirationage _strength _stimuluslocation _receiverlocation _tag _bsuccessfullysensed) (break `AIStimulus` Stimulus))
  (`|ExecutionSequence`
    (:`then_0`
      (bind _returnvalue (`AIPerceptionSystem.GetSenseClassForStimulus` Stimulus))
      (if (== _returnvalue "/Script/AIModule.AISense_Sight")
        (if (== Actor (`GameplayStatics.GetPlayerPawn` 0))
          (`|ExecutionSequence`
            (:`then_0`
              (`BlackboardComponent.SetValueAsObject` (`AIBlueprintHelperLibrary.GetBlackboard` null) "TargetActor" (select `bool` _bsuccessfullysensed :`true` Actor :!type "Object Object Reference")))
            (:`then_1`
              (if (not _bsuccessfullysensed)
                (`BlackboardComponent.SetValueAsVector` (`AIBlueprintHelperLibrary.GetBlackboard` null) "LastSeenLocation" _stimuluslocation)))))))
    (:`then_1`
      (bind _returnvalue_2 (`AIPerceptionSystem.GetSenseClassForStimulus` Stimulus))
      (if (== _returnvalue_2 "/Script/AIModule.AISense_Hearing")
        (`BlackboardComponent.SetValueAsVector` (`AIBlueprintHelperLibrary.GetBlackboard` null) "HearingNoiseLocation" (`.StimulusLocation` (break `AIStimulus` Stimulus)))))))

(fn `UserConstructionScript`)